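; Player pawn that fires a physics-driven Bullet from its barrel on left mouse click and reports the XP earned from hits.
; Each click spawns a scaled-down Bullet at BarrelPivot and applies an impulse to its Sphere along the pivot's forward vector.
; The pawn binds to each bullet's OnHitOfBullet event dispatcher, whose XP value it only prints to screen, without storing it.
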(event Custom|OnHit_Event
  (params (XP :type Float%20%28double-precision%29))
  (Development|PrintString (Utilities|String|Append "Player get XP:  " (Utilities|String|ToString(Float) XP))))

(event EventBeginPlay)

(event Collision|EventActorBeginOverlap
  (params (OtherActor :type Actor%20Object%20Reference)))

(event EventTick
  (params (DeltaSeconds :type Float%20%28single-precision%29)))

(event Input|MouseEvents|LeftMouseButton
  (params (Key :type Key%20Structure :default "None"))
  (:Pressed
    (bind _returnvalue (Game|SpawnActorfromClass "/Game/Blueprints/Bullet.Bullet_C" (Math|Transform|MakeTransform (Transformation|GetWorldLocation (Variables|Default|GetBarrelPivot)) "0, 0, 0" "0.100000,0.100000,0.100000") "AlwaysSpawn" "MultiplyWithRoot" 0 0))
    (Physics|AddImpulse (Variables|/Game/Blueprints/Bullet.Bullet_C|GetSphere _returnvalue) (* (Math|Vector|GetForwardVector (Variables|Default|GetBarrelPivot)) 1e+03) "None" false)
    (EventDispatchers|AssignOnHitOfBullet _returnvalue (delegate Custom|OnHit_Event))))

(fn ConstructionScript)