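; AlarmBase is an alarm actor that sounds on a timer and shuts down when a pawn reaches it.
; After play begins, a short delay leads to a Noise call, and a Pawn overlapping its Box calls Shutdown.
; Noise and Shutdown have no bodies in this Blueprint.
; The Swim event, empty NewFunc and counter-printing Reusable function are leftover scaffolding outside the alarm flow.
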(event OnComponentBeginOverlap(Box)
  (params (OverlappedComponent :type Primitive%20Component%20Object%20Reference) (OtherActor :type Actor%20Object%20Reference) (OtherComp :type Primitive%20Component%20Object%20Reference) (OtherBodyIndex :type Integer) (bFromSweep :type Boolean) (SweepResult :type Hit%20Result%20Structure%20%28by%20ref%29))
  (Utilities|Casting|CastToPawn OtherActor)
  (CallFunction|Shutdown))

(event EventBeginPlay
  (Utilities|FlowControl|Delay 2.0)
  (CallFunction|Noise))

(event Collision|EventActorBeginOverlap
  (params (OtherActor :type Actor%20Object%20Reference)))

(event EventTick
  (params (DeltaSeconds :type Float%20%28single-precision%29)))

(event Custom|Swim
  (CallFunction|NewFunc))

(fn ConstructionScript)

(fn Reusable
  ;[1 0 0.75] All of this code disabled
  (bind _result (Math|Integer|IncrementInt (Variables|Default|GetCount))
    (:%20%20
      (Development|PrintString (Utilities|String|ToString(Integer) _result) true true "(R=1.000000,G=0.000000,B=0.205652,A=1.000000)" 1e+01 "2"))))

(fn NewFunc)