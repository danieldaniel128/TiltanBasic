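; Shooter pawn blueprint that holds weapons as child actors and handles weapon switching and attacking.
; PickWeapon maps a weapon type to its child actor, adds it uniquely to WeaponInventory, hides every inventory weapon, then unhides the selected one.
; The Machinegun option is unconnected, and no current weapon is saved.
; Attack therefore always sends AttackMessage to the Rifle, a placeholder noted for replacement with the current weapon.
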(event Custom|Attack
  (Class|BPIWeapon|Attack(Message) (Variables|/Script/Engine.ChildActorComponent|GetChildActor (Variables|Default|GetRifle))))

(event Custom|PickWeapon
  (params (Type :type E_WeaponType%20Enum :default "NewEnumerator0"))
  (bind _shotgun (Variables|Default|GetShotgun))
  (bind _rifle (Variables|Default|GetRifle))
  (bind _returnvalue (Utilities|Select :Index Type :NewEnumerator0 _shotgun :NewEnumerator1 _rifle :NewEnumerator2 0))
  (bind _childactor (Variables|/Script/Engine.ChildActorComponent|GetChildActor _returnvalue))
  (Utilities|Array|AddUnique (Variables|Default|GetWeaponInventory) _childactor)
  (for _array_element (Variables|Default|GetWeaponInventory)
    (Rendering|SetActorHiddenInGame _array_element true))
  (Rendering|SetActorHiddenInGame _childactor false))

(event EventBeginPlay)

(fn ConstructionScript)