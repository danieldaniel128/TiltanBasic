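; BP_ShootableWeapon is a shooter weapon that can be picked up and fires physical bullets.
; Attack checks and decrements ammo, then spawns a scaled-down bullet at the barrel pivot and launches it with a forward impulse.
; It binds to each bullet's hit dispatcher to print the XP earned.
; Player overlap with the mesh passes the weapon type to Pawn_New's PickWeapon, then destroys the actor.
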(event OnComponentBeginOverlap(SkeletalMesh)
  (params (OverlappedComponent :type Primitive%20Component%20Object%20Reference) (OtherActor :type Actor%20Object%20Reference) (OtherComp :type Primitive%20Component%20Object%20Reference) (OtherBodyIndex :type Integer) (bFromSweep :type Boolean) (SweepResult :type Hit%20Result%20Structure%20%28by%20ref%29))
  (if (== OtherActor (Game|GetPlayerCharacter 0))
    (CallFunction|Pick)))

(event Custom|OnHit_Event
  (params (XP :type Float%20%28double-precision%29))
  (Development|PrintText "Hit a Target" true true "(R=0.926786,G=1.000000,B=0.000000,A=1.000000)")
  (Development|PrintString (Utilities|String|Append "Player get XP:  " (Utilities|String|ToString(Float) XP))))

(event EventPick
  (bind _aspawn_new (Utilities|Casting|CastToPawn_New (Game|GetPlayerCharacter 0)))
  (Default|PickWeapon _aspawn_new (Variables|Default|GetWeaponType))
  (Actor|DestroyActor))

(event EventAttack
  (if (== (Variables|Default|GetAmmoCount) 0)
    (Development|PrintString "No Bullets")
    (else
      (bind _result (Math|Integer|DecrementInt (Variables|Default|GetAmmoCount))
        (:%20%20
          (Development|PrintString (Utilities|String|ToString(Integer) _result))
          (bind _returnvalue (Game|SpawnActorfromClass "/Game/Shooter/Blueprints/Bullet.Bullet_C" (Math|Transform|MakeTransform (Transformation|GetWorldLocation (Variables|Default|GetBarrelPivot)) "0, 0, 0" "0.100000,0.100000,0.100000") "AlwaysSpawn" "MultiplyWithRoot" 0 0))
          (Physics|AddImpulse (Variables|/Game/Shooter/Blueprints/Bullet.Bullet_C|GetSphere _returnvalue) (* (Math|Vector|GetForwardVector (Variables|Default|GetBarrelPivot)) 1e+03) "None" false)
          (EventDispatchers|AssignOnHitOfBullet _returnvalue (delegate Custom|OnHit_Event)))))))

(fn ConstructionScript)