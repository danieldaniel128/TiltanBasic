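; EnterCabin is a trigger actor that reveals an alarm object's mesh when a pawn enters its Box.
; At BeginPlay it caches all AlarmBase actors tagged RightCube in Cubes.
; A pawn overlapping the Box makes only the first cached actor's StaticMesh visible, with nothing to hide it again.
; Non-pawn overlaps and Box hits just print debug strings.
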(event OnComponentBeginOverlap(Box)
  (params (OverlappedComponent :type Primitive%20Component%20Object%20Reference) (OtherActor :type Actor%20Object%20Reference) (OtherComp :type Primitive%20Component%20Object%20Reference) (OtherBodyIndex :type Integer) (bFromSweep :type Boolean) (SweepResult :type Hit%20Result%20Structure%20%28by%20ref%29))
  (bind _cubes (Variables|Default|GetCubes))
  (Utilities|Casting|CastToPawn OtherActor
    (:then
      ;[1 1 1] Comment
      (if (> (Utilities|Array|Length _cubes) 0)
        (Rendering|SetVisibility (Variables|/Game/Shooter/Blueprints/AlarmBase.AlarmBase_C|GetStaticMesh (Utilities|Array|Get(acopy) _cubes)) true false)))
    (:CastFailed
      (Development|PrintString "No a pawn!"))))

(event OnComponentHit(Box)
  (params (HitComponent :type Primitive%20Component%20Object%20Reference) (OtherActor :type Actor%20Object%20Reference) (OtherComp :type Primitive%20Component%20Object%20Reference) (NormalImpulse :type Vector :default "0, 0, 0") (Hit :type Hit%20Result%20Structure%20%28by%20ref%29))
  (Development|PrintString "Hello"))

(event Collision|EventActorBeginOverlap
  (params (OtherActor :type Actor%20Object%20Reference)))

(event EventTick
  (params (DeltaSeconds :type Float%20%28single-precision%29)))

(event EventBeginPlay
  (bind _outactors (Actor|GetAllActorsOfClasswithTag "/Game/Shooter/Blueprints/AlarmBase.AlarmBase_C" "RightCube"))
  (Variables|Default|SetCubes _outactors))

(fn ConstructionScript)