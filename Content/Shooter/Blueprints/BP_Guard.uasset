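; BP_Guard is a guard pawn that turns to face the player when it sees them directly ahead.
; Each Tick, a short debug-drawn Visibility line trace runs forward from HeadPivot, and a hit on the player pawn calls RotateTowardPlayer, which snaps rotation via look-at.
; An AI Move To chain toward TargetPoint, then the player, is disconnected and never runs.
; GetXP is a stub returning zero.
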(event EventBeginPlay)

(event EventTick
  (params (DeltaSeconds :type Float%20%28single-precision%29))
  (bind _headpivot (Variables|Default|GetHeadPivot))
  (bind _returnvalue (Transformation|GetWorldLocation _headpivot))
  (bind _outhit (Collision|LineTraceByChannel _returnvalue (+ _returnvalue (* (Math|Vector|GetForwardVector _headpivot) 5e+02)) "TraceTypeQuery1" false 0 "ForOneFrame"))
  (if (== (.HitActor (Collision|BreakHitResult _outhit)) (Game|Player|GetPlayerPawn 0))
    (CallFunction|RotateTowardPlayer)
    (Development|PrintString "Rotate to player")))

(fn ConstructionScript)

(fn GetXP
  (return 0.0))

(fn RotateTowardPlayer
  (Transformation|SetActorRotation (Math|Rotator|FindLookatRotation (Transformation|GetActorLocation) (Transformation|GetActorLocation (Game|Player|GetPlayerPawn 0)))))