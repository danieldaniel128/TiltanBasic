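; PC_New is a player controller that turns Enhanced Input actions into shooter pawn controls.
; On BeginPlay it adds the IMC_Override mapping context.
; Move, look with inverted pitch input, and jump act on player 0's pawn or character, while shoot casts to Pawn_New and calls Attack.
; Crouch is hold-based, with a debug print on press; an unconnected toggle-crouch branch never runs.
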(event Input|EnhancedActionEvents|EnhancedInputActionIA_ShootNew
  (params (ActionValue :type Boolean) (ElapsedSeconds :type Float%20%28double-precision%29) (TriggeredSeconds :type Float%20%28double-precision%29) (InputAction :type Input%20Action%20Object%20Reference :default "/Game/Shooter/Input/Actions/IA_ShootNew.IA_ShootNew"))
  (bind _aspawn_new (Utilities|Casting|CastToPawn_New (Game|Player|GetPlayerPawn 0)))
  (Default|Attack _aspawn_new))

(event Input|EnhancedActionEvents|EnhancedInputActionIA_JumpNew
  (params (ActionValue :type Boolean) (ElapsedSeconds :type Float%20%28double-precision%29) (TriggeredSeconds :type Float%20%28double-precision%29) (InputAction :type Input%20Action%20Object%20Reference :default "/Game/Shooter/Input/Actions/IA_JumpNew.IA_JumpNew"))
  (Character|Jump (Game|GetPlayerCharacter 0)))

(event Input|EnhancedActionEvents|EnhancedInputActionIA_LookNew
  (params (ActionValue :type Vector%202D%20Structure) (ElapsedSeconds :type Float%20%28double-precision%29) (TriggeredSeconds :type Float%20%28double-precision%29) (InputAction :type Input%20Action%20Object%20Reference :default "/Game/Shooter/Input/Actions/IA_LookNew.IA_LookNew"))
  (bind _returnvalue (Game|Player|GetPlayerPawn 0))
  (bind (_x _y) (Math|Vector2D|BreakVector2D ActionValue))
  (Pawn|Input|AddControllerYawInput _returnvalue _x)
  (Pawn|Input|AddControllerPitchInput _returnvalue (* _y -1.0)))

(event Input|EnhancedActionEvents|EnhancedInputActionIA_MoveNew
  (params (ActionValue :type Vector%202D%20Structure) (ElapsedSeconds :type Float%20%28double-precision%29) (TriggeredSeconds :type Float%20%28double-precision%29) (InputAction :type Input%20Action%20Object%20Reference :default "/Game/Shooter/Input/Actions/IA_MoveNew.IA_MoveNew"))
  (bind (_x _y) (Math|Vector2D|BreakVector2D ActionValue))
  (bind _returnvalue (Game|Player|GetPlayerPawn 0))
  (Pawn|Input|AddMovementInput _returnvalue (Transformation|GetActorForwardVector _returnvalue) _y false)
  (Pawn|Input|AddMovementInput _returnvalue (Transformation|GetActorRightVector _returnvalue) _x false))

(event Input|EnhancedActionEvents|EnhancedInputActionIA_CrouchNew
  (params (ActionValue :type Boolean) (ElapsedSeconds :type Float%20%28double-precision%29) (TriggeredSeconds :type Float%20%28double-precision%29) (InputAction :type Input%20Action%20Object%20Reference :default "/Game/Shooter/Input/Actions/IA_CrouchNew.IA_CrouchNew"))
  (:Started
    (Development|PrintString "Crouch")
    (Character|Crouch (Game|GetPlayerCharacter 0)))
  (:Completed
    (Character|UnCrouch (Game|GetPlayerCharacter 0))))

(event EventBeginPlay
  (Input|AddMappingContext (PlayerController|LocalPlayerSubsystems|GetEnhancedInputLocalPlayerSubsystem self) "/Game/Shooter/Input/IMC_Override.IMC_Override" 0 "(bIgnoreAllPressedKeysUntilRelease=True,bForceImmediately=False,bNotifyUserSettings=False)"))

(event EventTick
  (params (DeltaSeconds :type Float%20%28single-precision%29)))

(fn ConstructionScript)