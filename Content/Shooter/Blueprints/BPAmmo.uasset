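; BPAmmo is an ammo pickup actor with a random AmmoAmount, rolled between Min and Max on BeginPlay.
; When the player character overlaps its Cylinder, Pick casts to Pawn_New and compares WeaponType with the current weapon's.
; On a match it prints the amount, adds the weapon's AmmoCount into its own AmmoAmount and destroys itself.
; The weapon's AmmoCount is never written here.
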(event OnComponentBeginOverlap(Cylinder)
  (params (OverlappedComponent :type Primitive%20Component%20Object%20Reference) (OtherActor :type Actor%20Object%20Reference) (OtherComp :type Primitive%20Component%20Object%20Reference) (OtherBodyIndex :type Integer) (bFromSweep :type Boolean) (SweepResult :type Hit%20Result%20Structure%20%28by%20ref%29))
  (if (== OtherActor (Game|GetPlayerCharacter 0))
    (CallFunction|Pick)))

(event EventBeginPlay
  (Variables|Default|SetAmmoAmount (Math|Random|RandomIntegerinRange (Variables|Default|GetMin) (Variables|Default|GetMax))))

(event EventPick
  (bind _aspawn_new (Utilities|Casting|CastToPawn_New (Game|GetPlayerCharacter 0)))
  (if (== (Variables|Default|GetweaponType) (Math|Conversions|ToInteger(Byte) (Variables|/Game/Shooter/Blueprints/BP_ShootableWeapon.BP_ShootableWeapon_C|GetWeaponType (Variables|/Game/Shooter/Blueprints/Pawn_New.Pawn_New_C|GetCurrentWeapon _aspawn_new))))
    (Development|PrintString "collected ammo:")
    (Development|PrintString (Utilities|String|ToString(Integer) (Variables|Default|GetAmmoAmount)))
    (Variables|Default|SetAmmoAmount (+ (Variables|Default|GetAmmoAmount) (Variables|/Game/Shooter/Blueprints/BP_ShootableWeapon.BP_ShootableWeapon_C|GetAmmoCount (Variables|/Game/Shooter/Blueprints/Pawn_New.Pawn_New_C|GetCurrentWeapon _aspawn_new))))
    (Actor|DestroyActor)))

(fn ConstructionScript)